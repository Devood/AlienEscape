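; Sci-fi interior sliding door that opens when something overlaps its trigger and closes when the overlap ends.
; A timeline lerps the door mesh's relative location between closed and open positions, playing forward on entry and reversing on exit.
; Entry also activates two steam components.
; The open sound plays as quiet 2D audio on every timeline update, so it retriggers throughout movement in both directions.
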(event OnComponentBeginOverlap(Trigger)
  (params (OverlappedComponent :type Primitive%20Component%20Object%20Reference) (OtherActor :type Actor%20Object%20Reference) (OtherComp :type Primitive%20Component%20Object%20Reference) (OtherBodyIndex :type Integer) (bFromSweep :type Boolean) (SweepResult :type Hit%20Result%20Structure%20%28by%20ref%29))
  (Components|Activation|Activate (Variables|Default|GetSteamDoor) false)
  (bind _doorposition (Timeline|Timeline_0 Play)
    (:Update
      (Transformation|SetRelativeLocation (Variables|Default|GetDoor_Small_A) (Math|Vector|Lerp(Vector) (Variables|Door|GetDoorClosed) (Variables|Door|GetDoorOpen) _doorposition) false false)
      (Audio|PlaySound2D "/Game/FirstPerson/Audio/DoorOpen.DoorOpen" 0.15 1.0 0.0 0 0))))

(event OnComponentEndOverlap(Trigger)
  (params (OverlappedComponent :type Primitive%20Component%20Object%20Reference) (OtherActor :type Actor%20Object%20Reference) (OtherComp :type Primitive%20Component%20Object%20Reference) (OtherBodyIndex :type Integer))
  (bind _doorposition (Timeline|Timeline_0 Reverse)
    (:Update
      (Transformation|SetRelativeLocation (Variables|Default|GetDoor_Small_A) (Math|Vector|Lerp(Vector) (Variables|Door|GetDoorClosed) (Variables|Door|GetDoorOpen) _doorposition) false false)
      (Audio|PlaySound2D "/Game/FirstPerson/Audio/DoorOpen.DoorOpen" 0.15 1.0 0.0 0 0))))

(fn ConstructionScript)